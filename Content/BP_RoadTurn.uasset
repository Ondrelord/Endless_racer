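; BP_RoadTurn is a turn road tile for a racer game that spawns tiles as the vehicle progresses.
; On BeginPlay it spawns a coin at one of three spawn points chosen at random.
; When the vehicle overlaps EndTileTrigger, it asks RacerGameMode to add a random tile, then after a short delay destroys itself and its coin.
; GetAttachTransform exposes the AttachPoint world transform.
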(event OnComponentBeginOverlap(EndTileTrigger)
  (params (OverlappedComponent :type Primitive%20Component%20Object%20Reference) (OtherActor :type Actor%20Object%20Reference) (OtherComp :type Primitive%20Component%20Object%20Reference) (OtherBodyIndex :type Integer) (bFromSweep :type Boolean) (SweepResult :type Hit%20Result%20Structure%20%28by%20ref%29))
  (Utilities|Casting|CastToVehicleBlueprint OtherActor)
  (bind _asracer_game_mode (Utilities|Casting|CastToRacerGameMode (Game|GetGameMode)))
  (Default|AddRandomRoadTile _asracer_game_mode)
  (Utilities|FlowControl|Delay 2.0)
  (Actor|DestroyActor)
  (if (Utilities|IsValid (stale EventBeginPlay _returnvalue))
    (Actor|DestroyActor (stale EventBeginPlay _returnvalue))))

(event EventBeginPlay
  (bind _returnvalue (Game|SpawnActorfromClass "/Game/BP_Coin.BP_Coin_C" (Transformation|GetWorldTransform (Utilities|Array|Get(acopy) (Utilities|Array|MakeArray (Variables|Default|GetSpawn%20Coin%20L) (Variables|Default|GetSpawn%20Coin%20R) (Variables|Default|GetSpawn%20Coin)) (Math|Random|RandomIntegerinRange 0 2))) "Undefined" 0 0)))

(event Collision|EventActorBeginOverlap
  (params (OtherActor :type Actor%20Object%20Reference)))

(event EventTick
  (params (DeltaSeconds :type Float%20%28single-precision%29)))

(fn ConstructionScript)

(fn GetAttachTransform
  (return (Transformation|GetWorldTransform (Variables|Default|GetAttachPoint))))
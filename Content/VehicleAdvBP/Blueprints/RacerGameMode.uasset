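; Game mode for a procedural road racer that builds the track, keeps score and reloads the level after the player falls below a death depth.
; BeginPlay lays straight tiles, each chained to the previous attach transform.
; AddRandomRoadTile appends straights, turns, S-turns, jumps or loops by cascading random rolls, mirroring via negative Y scale and using TurnCounter to restrict turns.
; AddScore raises a combo multiplier that Tick resets when its timer expires.
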(event EventBeginPlay
  (for _index (range 0 5)
    (CallFunction|AddFloorTile)))

(event EventTick
  (params (DeltaSeconds :type Float%20%28single-precision%29))
  (if (<= (Variables|Default|GetScoreMultiplierTimer) 0.0)
    (Variables|Default|SetScoreMultiplier 1)
    (else
      (Variables|Default|SetScoreMultiplierTimer (- (Variables|Default|GetScoreMultiplierTimer) DeltaSeconds))))
  (if (<= (.Z (Math|Vector|BreakVector (Transformation|GetActorLocation (Game|Player|GetPlayerPawn 0)))) (Variables|Default|GetDeathDepth))
    (Utilities|FlowControl|Delay 2.0)
    (bind _returnvalue (Game|GetCurrentLevelName true))
    (Game|OpenLevel(byName) (Utilities|String|StringToName _returnvalue))))

(fn ConstructionScript)

(fn AddFloorTile
  (bind _returnvalue (Game|SpawnActorfromClass "/Game/BP_RoadStraight.BP_RoadStraight_C" (Variables|Default|GetNextSpawnPoint) "Undefined" 0 0))
  (bind _asbp_road_straight (Utilities|Casting|CastToBP_RoadStraight _returnvalue))
  (bind _attachpoint_transform (Default|GetAttachTransform _asbp_road_straight))
  (Variables|Default|SetNextSpawnPoint _attachpoint_transform))

(fn AddRandomRoadTile
  (bind _returnvalue (Math|Random|RandomBool))
  (bind _returnvalue_2 (Math|Random|RandomFloat))
  (bind _returnvalue_3 (Math|Float|SelectFloat -1.0 1.0 _returnvalue))
  (bind _returnvalue_4 (Math|Float|Round _returnvalue_3))
  (bind _returnvalue_5 (Class|KismetMathLibrary|SignOfInteger _returnvalue_4))
  (if (< _returnvalue_2 0.4)
    (bind _returnvalue_6 (Game|SpawnActorfromClass "/Game/BP_RoadStraight.BP_RoadStraight_C" (Variables|Default|GetNextSpawnPoint) "Undefined" 0 0))
    (bind _attachpoint_transform (Default|GetAttachTransform _returnvalue_6))
    (Variables|Default|SetNextSpawnPoint _attachpoint_transform)
    (elif (< _returnvalue_2 0.7)
      (if (< (Math|Integer|Absolute(Integer) (+ (Variables|Default|GetTurnCounter) _returnvalue_5)) 3)
        (bind _returnvalue_7 (Game|SpawnActorfromClass "/Game/BP_RoadTurn.BP_RoadTurn_C" (Math|Transform|MakeTransform (.Location (Math|Transform|BreakTransform (Variables|Default|GetNextSpawnPoint))) (.Rotation (Math|Transform|BreakTransform (Variables|Default|GetNextSpawnPoint))) (Math|Vector|MakeVector (.X (Math|Vector|BreakVector (.Scale (Math|Transform|BreakTransform (Variables|Default|GetNextSpawnPoint))))) (* (.Y (Math|Vector|BreakVector (.Scale (Math|Transform|BreakTransform (Variables|Default|GetNextSpawnPoint))))) _returnvalue_3) (.Z (Math|Vector|BreakVector (.Scale (Math|Transform|BreakTransform (Variables|Default|GetNextSpawnPoint))))))) "Undefined" 0 0))
        (bind _attachpoint_transform_2 (Default|GetAttachTransform _returnvalue_7))
        (Variables|Default|SetNextSpawnPoint _attachpoint_transform_2)
        (Variables|Default|SetTurnCounter (+ (Class|KismetMathLibrary|SignOfInteger (Variables|Default|GetTurnCounter)) _returnvalue_5))
        (else
          (CallFunction|AddRandomRoadTile)))
      (elif (< _returnvalue_2 0.85)
        (bind _returnvalue_8 (Game|SpawnActorfromClass "/Game/BP_RoadSTurn.BP_RoadSTurn_C" (Math|Transform|MakeTransform (.Location (Math|Transform|BreakTransform (Variables|Default|GetNextSpawnPoint))) (.Rotation (Math|Transform|BreakTransform (Variables|Default|GetNextSpawnPoint))) (Math|Vector|MakeVector (.X (Math|Vector|BreakVector (.Scale (Math|Transform|BreakTransform (Variables|Default|GetNextSpawnPoint))))) (* (.Y (Math|Vector|BreakVector (.Scale (Math|Transform|BreakTransform (Variables|Default|GetNextSpawnPoint))))) _returnvalue_3) (.Z (Math|Vector|BreakVector (.Scale (Math|Transform|BreakTransform (Variables|Default|GetNextSpawnPoint))))))) "Undefined" 0 0))
        (bind _attachpoint_transform_3 (Default|GetAttachTransform _returnvalue_8))
        (Variables|Default|SetNextSpawnPoint _attachpoint_transform_3)
        (elif (< _returnvalue_2 0.93)
          (bind _returnvalue_9 (Game|SpawnActorfromClass "/Game/BP_RoadJump.BP_RoadJump_C" (Variables|Default|GetNextSpawnPoint) "Undefined" 0 0))
          (bind _attachpoint_transform_4 (Default|GetAttachTransform _returnvalue_9))
          (Variables|Default|SetNextSpawnPoint _attachpoint_transform_4)
          (else
            (bind _returnvalue_10 (Game|SpawnActorfromClass "/Game/BP_RoadLoop.BP_RoadLoop_C" (Math|Transform|MakeTransform (.Location (Math|Transform|BreakTransform (Variables|Default|GetNextSpawnPoint))) (.Rotation (Math|Transform|BreakTransform (Variables|Default|GetNextSpawnPoint))) (Math|Vector|MakeVector (.X (Math|Vector|BreakVector (.Scale (Math|Transform|BreakTransform (Variables|Default|GetNextSpawnPoint))))) (* (.Y (Math|Vector|BreakVector (.Scale (Math|Transform|BreakTransform (Variables|Default|GetNextSpawnPoint))))) _returnvalue_3) (.Z (Math|Vector|BreakVector (.Scale (Math|Transform|BreakTransform (Variables|Default|GetNextSpawnPoint))))))) "Undefined" 0 0))
            (bind _attachpoint_transform_5 (Default|GetAttachTransform _returnvalue_10))
            (Variables|Default|SetNextSpawnPoint _attachpoint_transform_5)))))))

(fn AddScore
  (Variables|Default|SetScore (+ (Variables|Default|GetScore) (Variables|Default|GetScoreMultiplier)))
  (bind _result (Math|Integer|IncrementInt (Variables|Default|GetScoreMultiplier))
    (:%20%20
      (Variables|Default|SetScoreMultiplier _result)
      (Variables|Default|SetScoreMultiplierTimer 2.0))))